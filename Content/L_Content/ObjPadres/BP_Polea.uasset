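; Pulley actor that lowers its Box platform and raises SM2 while an actor tagged Heavy rests on the Box.
; Overlap begin starts a looping timer that interpolates both parts at constant speed and snaps the BP_HeavyObj onto the Box.
; Overlap end swaps to a return timer toward the Z positions saved at BeginPlay.
; Timers stop on truncated Z comparisons; the return check compares against the negated initial Box Z.
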(event OnComponentBeginOverlap(Box)
  (params (OverlappedComponent :type Primitive%20Component%20Object%20Reference) (OtherActor :type Actor%20Object%20Reference) (OtherComp :type Primitive%20Component%20Object%20Reference) (OtherBodyIndex :type Integer) (bFromSweep :type Boolean) (SweepResult :type Hit%20Result%20Structure%20%28by%20ref%29))
  (if (Actor|ActorHasTag OtherActor "Heavy")
    (Utilities|Time|ClearandInvalidateTimerbyHandle (Variables|Default|GetUpHandleTimer))
    (bind _asbp_heavy_obj (Utilities|Casting|CastToBP_HeavyObj OtherActor))
    (Variables|Default|SetAs%20BP%20Heavy%20Obj _asbp_heavy_obj)
    (bind _returnvalue (Utilities|Time|SetTimerbyEvent (delegate Custom|CE_Down) 0.01 true))
    (Variables|Default|SetDownHandleTimer _returnvalue)))

(event OnComponentEndOverlap(Box)
  (params (OverlappedComponent :type Primitive%20Component%20Object%20Reference) (OtherActor :type Actor%20Object%20Reference) (OtherComp :type Primitive%20Component%20Object%20Reference) (OtherBodyIndex :type Integer))
  (if (Actor|ActorHasTag OtherActor "Heavy")
    (Utilities|Time|ClearandInvalidateTimerbyHandle (Variables|Default|GetDownHandleTimer))
    (bind _returnvalue (Utilities|Time|SetTimerbyEvent (delegate Custom|CE_Return) 0.01 true))
    (Variables|Default|SetUpHandleTimer _returnvalue)))

(event Custom|CE_Down
  (bind _returnvalue (Utilities|Time|GetWorldDeltaSeconds))
  (bind _box (Variables|Default|GetBox))
  (bind _zrelativelocdownsm1 (Variables|Default|GetZrelativeLocDownSM1))
  (bind _sm2 (Variables|Default|GetSM2))
  (bind _speed (Variables|Default|GetSpeed))
  (bind _relativelocation (Variables|/Script/Engine.SceneComponent|GetRelativeLocation _box))
  (bind _relativelocation_2 (Variables|/Script/Engine.SceneComponent|GetRelativeLocation _sm2))
  (bind _returnvalue_2 (Math|Interpolation|FInterptoConstant (.z _relativelocation) _zrelativelocdownsm1 _returnvalue _speed))
  (bind _as_bp_heavy_obj (Variables|Default|GetAs%20BP%20Heavy%20Obj)
    (:then
      (Transformation|SetActorLocation _as_bp_heavy_obj (+ (Transformation|GetWorldLocation (Variables|Default|GetBox)) "0.000000,0.000000,10.000000") false false)
      (Transformation|SetRelativeLocation _box (Math|Vector|MakeVector (.x _relativelocation) (.y _relativelocation) _returnvalue_2) false false)
      (if (== (Math|Float|Truncate _returnvalue_2) (Math|Float|Truncate _zrelativelocdownsm1))
        (Utilities|Time|ClearandInvalidateTimerbyHandle (Variables|Default|GetDownHandleTimer))
        (else
          (Transformation|SetRelativeLocation _sm2 (Math|Vector|MakeVector (.x _relativelocation_2) (.y _relativelocation_2) (Math|Interpolation|FInterptoConstant (.z _relativelocation_2) (Variables|Default|GetZrelativeLocUpSm2) (Utilities|Time|GetWorldDeltaSeconds) (Variables|Default|GetSpeed))) false false))))
    (:else)))

(event Custom|CE_Return
  (bind _returnvalue (Utilities|Time|GetWorldDeltaSeconds))
  (bind _zrelativelocinitialsm1 (Variables|Default|GetZrelativeLocinitialSm1))
  (bind _box (Variables|Default|GetBox))
  (bind _speed (Variables|Default|GetSpeed))
  (bind _sm2 (Variables|Default|GetSM2))
  (bind _relativelocation (Variables|/Script/Engine.SceneComponent|GetRelativeLocation _sm2))
  (bind _relativelocation_2 (Variables|/Script/Engine.SceneComponent|GetRelativeLocation _box))
  (bind _returnvalue_2 (Math|Interpolation|FInterptoConstant (.z _relativelocation_2) _zrelativelocinitialsm1 _returnvalue _speed))
  (Transformation|SetRelativeLocation _box (Math|Vector|MakeVector (.x _relativelocation_2) (.y _relativelocation_2) _returnvalue_2) false false)
  (if (== (Math|Float|Truncate _returnvalue_2) (Math|Float|Truncate (* _zrelativelocinitialsm1 -1.0)))
    (Utilities|Time|ClearandInvalidateTimerbyHandle (Variables|Default|GetUpHandleTimer))
    (else
      (Transformation|SetRelativeLocation _sm2 (Math|Vector|MakeVector (.x _relativelocation) (.y _relativelocation) (Math|Interpolation|FInterptoConstant (.z _relativelocation) (Variables|Default|GetZrelativeLocinitial) (Utilities|Time|GetWorldDeltaSeconds) (Variables|Default|GetSpeed))) false false))))

(event EventBeginPlay
  (Variables|Default|SetZrelativeLocinitialSm1 (.z (Variables|/Script/Engine.SceneComponent|GetRelativeLocation (Variables|Default|GetBox))))
  (Variables|Default|SetZrelativeLocinitial (.z (Variables|/Script/Engine.SceneComponent|GetRelativeLocation (Variables|Default|GetSM2)))))

(event Collision|EventActorBeginOverlap
  (params (OtherActor :type Actor%20Object%20Reference)))

(event EventTick
  (params (DeltaSeconds :type Float%20%28single-precision%29)))

(fn ConstructionScript)