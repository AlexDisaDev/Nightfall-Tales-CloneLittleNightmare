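; Interactive door actor that the player can open once, moving the character into place as it swings.
; Its box overlap sets the player's NearDoor flag and passes the door to the character via AttachmentMessage.
; Activate runs a Location timeline that lerps the character to the Arrow's position and door's rotation while turning the door's yaw to TargetRot.
; The timeline update restores walking, collision and CanMove once playback stops.
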(event OnComponentBeginOverlap(Box)
  (params (OverlappedComponent :type Primitive%20Component%20Object%20Reference) (OtherActor :type Actor%20Object%20Reference) (OtherComp :type Primitive%20Component%20Object%20Reference) (OtherBodyIndex :type Integer) (bFromSweep :type Boolean) (SweepResult :type Hit%20Result%20Structure%20%28by%20ref%29))
  (if (Actor|ActorHasTag OtherActor "Player")
    (bind _asbp_third_person_character (Utilities|Casting|CastToBP_ThirdPersonCharacter OtherActor))
    (Variables|/Game/L_Content/Character/BP_ThirdPersonCharacter.BP_ThirdPersonCharacter_C|SetbNearDoor _asbp_third_person_character true)
    (Class|BPIDoors|Attachment(Message) _asbp_third_person_character self)))

(event OnComponentEndOverlap(Box)
  (params (OverlappedComponent :type Primitive%20Component%20Object%20Reference) (OtherActor :type Actor%20Object%20Reference) (OtherComp :type Primitive%20Component%20Object%20Reference) (OtherBodyIndex :type Integer))
  (if (Actor|ActorHasTag OtherActor "Player")
    (bind _asbp_third_person_character (Utilities|Casting|CastToBP_ThirdPersonCharacter OtherActor))
    (Variables|/Game/L_Content/Character/BP_ThirdPersonCharacter.BP_ThirdPersonCharacter_C|SetbNearDoor _asbp_third_person_character false)))

(event Custom|CE_DoorRot
  (Utilities|FlowControl|Sequence))

(event EventBeginPlay)

(event Collision|EventActorBeginOverlap
  (params (OtherActor :type Actor%20Object%20Reference)))

(event EventTick
  (params (DeltaSeconds :type Float%20%28single-precision%29)))

(event EventActivate
  (params (actor :type BP%20Third%20Person%20Character%20Object%20Reference) (Cam :type Camera%20Component%20Object%20Reference))
  (bind _door (Variables|Default|GetDoor))
  (bind _relativerotation (Variables|/Script/Engine.SceneComponent|GetRelativeRotation _door))
  (Utilities|FlowControl|DoOnce false
    (:Completed
      (Variables|Default|SetCam Cam)
      (Variables|Default|SetActor actor)
      (Utilities|FlowControl|Sequence
        (:then_1
          (bind _alpha (Timeline|Location Play)
            (:Update
              (Transformation|SetActorLocation (Variables|Default|GetActor) (Math|Vector|Lerp(Vector) (Transformation|GetActorLocation (Variables|Default|GetActor)) (Transformation|GetWorldLocation (Variables|Default|GetArrow)) (* _alpha (Variables|Default|GetActorTransformSpeed))) true false)
              (Transformation|SetActorRotation (Variables|Default|GetActor) (Math|Rotator|Lerp(Rotator) (Transformation|GetActorRotation (Variables|Default|GetActor)) (Transformation|GetWorldRotation (Variables|Default|GetDoor)) (* _alpha (Variables|Default|GetActorTransformSpeed)) true))
              (Transformation|SetRelativeRotation _door (Math|Rotator|MakeRotator (.roll _relativerotation) (.pitch _relativerotation) (Math|Float|Lerp (.yaw (Variables|/Script/Engine.SceneComponent|GetRelativeRotation (Variables|Default|GetDoor))) (Variables|Default|GettargetRot) (* _alpha (Variables|Default|GetDoorSpeed)))) false false)
              (if (not (Audio|Components|Audio|IsPlaying (Variables|GetLocation)))
                (Pawn|Components|CharacterMovement|SetMovementMode (Variables|/Script/Engine.Character|GetCharacterMovement (Variables|Default|GetActor)) "MOVE_Walking" 0)
                (Collision|SetActorEnableCollision (Variables|Default|GetActor) true)
                (Variables|/Game/L_Content/Character/BP_ThirdPersonCharacter.BP_ThirdPersonCharacter_C|SetCanMove (Variables|Default|GetActor) true)))))))))

(fn ConstructionScript)