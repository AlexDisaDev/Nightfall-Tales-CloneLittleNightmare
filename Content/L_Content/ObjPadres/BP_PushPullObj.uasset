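; Pushable and pullable object that the player moves along world X or Y, chosen by which of four side colliders they overlap.
; Overlaps register the character, side and facing arrow; AxisMovement then interpolates the object (Y clamped) and holds the character at that arrow.
; A box trace detects obstacles and blocks repeating the blocked side and direction, allowing pulling away.
; A retriggerable delay zeroes the character's animation axis when input stops.
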(event OnComponentBeginOverlap(collision)
  (params (OverlappedComponent :type Primitive%20Component%20Object%20Reference) (OtherActor :type Actor%20Object%20Reference) (OtherComp :type Primitive%20Component%20Object%20Reference) (OtherBodyIndex :type Integer) (bFromSweep :type Boolean) (SweepResult :type Hit%20Result%20Structure%20%28by%20ref%29))
  ;[1 1 1] inicio de overlap para poder interactuar
  (if (Actor|ActorHasTag OtherActor "player")
    (Variables|Default|SetIndexCollision 0)
    (bind _as_bp_third_person_character (Variables|Default|GetAs%20BP%20Third%20Person%20Character)
      (:then
        _)
      (:else
        (bind _asbp_third_person_character (Utilities|Casting|CastToBP_ThirdPersonCharacter OtherActor))
        (Variables|Default|SetAs%20BP%20Third%20Person%20Character _asbp_third_person_character)))
    (Variables|/Game/L_Content/Character/BP_ThirdPersonCharacter.BP_ThirdPersonCharacter_C|SetNearPushPullObject _as_bp_third_person_character true)
    (Variables|Default|SetisX?%20orY true)
    (Variables|/Game/L_Content/Character/BP_ThirdPersonCharacter.BP_ThirdPersonCharacter_C|SetBoxRotDirArrow (Variables|Default|GetAs%20BP%20Third%20Person%20Character) (Variables|Default|GetArrow))))

(event OnComponentBeginOverlap(collision3)
  (params (OverlappedComponent :type Primitive%20Component%20Object%20Reference) (OtherActor :type Actor%20Object%20Reference) (OtherComp :type Primitive%20Component%20Object%20Reference) (OtherBodyIndex :type Integer) (bFromSweep :type Boolean) (SweepResult :type Hit%20Result%20Structure%20%28by%20ref%29))
  ;[1 1 1] inicio de overlap para poder interactuar
  (if (Actor|ActorHasTag OtherActor "player")
    (Variables|Default|SetIndexCollision 3)
    (bind _as_bp_third_person_character (Variables|Default|GetAs%20BP%20Third%20Person%20Character)
      (:then
        _)
      (:else
        (bind _asbp_third_person_character (Utilities|Casting|CastToBP_ThirdPersonCharacter OtherActor))
        (Variables|Default|SetAs%20BP%20Third%20Person%20Character _asbp_third_person_character)))
    (Variables|/Game/L_Content/Character/BP_ThirdPersonCharacter.BP_ThirdPersonCharacter_C|SetNearPushPullObject _as_bp_third_person_character true)
    (Variables|Default|SetisX?%20orY false)
    (Variables|/Game/L_Content/Character/BP_ThirdPersonCharacter.BP_ThirdPersonCharacter_C|SetBoxRotDirArrow (Variables|Default|GetAs%20BP%20Third%20Person%20Character) (Variables|Default|GetArrow3))))

(event OnComponentBeginOverlap(collision1)
  (params (OverlappedComponent :type Primitive%20Component%20Object%20Reference) (OtherActor :type Actor%20Object%20Reference) (OtherComp :type Primitive%20Component%20Object%20Reference) (OtherBodyIndex :type Integer) (bFromSweep :type Boolean) (SweepResult :type Hit%20Result%20Structure%20%28by%20ref%29))
  ;[1 1 1] inicio de overlap para poder interactuar
  (if (Actor|ActorHasTag OtherActor "player")
    (Variables|Default|SetIndexCollision 1)
    (bind _as_bp_third_person_character (Variables|Default|GetAs%20BP%20Third%20Person%20Character)
      (:then
        _)
      (:else
        (bind _asbp_third_person_character (Utilities|Casting|CastToBP_ThirdPersonCharacter OtherActor))
        (Variables|Default|SetAs%20BP%20Third%20Person%20Character _asbp_third_person_character)))
    (Variables|/Game/L_Content/Character/BP_ThirdPersonCharacter.BP_ThirdPersonCharacter_C|SetNearPushPullObject _as_bp_third_person_character true)
    (Variables|Default|SetisX?%20orY true)
    (Variables|/Game/L_Content/Character/BP_ThirdPersonCharacter.BP_ThirdPersonCharacter_C|SetBoxRotDirArrow (Variables|Default|GetAs%20BP%20Third%20Person%20Character) (Variables|Default|GetArrow1))))

(event OnComponentBeginOverlap(collision2)
  (params (OverlappedComponent :type Primitive%20Component%20Object%20Reference) (OtherActor :type Actor%20Object%20Reference) (OtherComp :type Primitive%20Component%20Object%20Reference) (OtherBodyIndex :type Integer) (bFromSweep :type Boolean) (SweepResult :type Hit%20Result%20Structure%20%28by%20ref%29))
  ;[1 1 1] inicio de overlap para poder interactuar
  (if (Actor|ActorHasTag OtherActor "player")
    (Variables|Default|SetIndexCollision 2)
    (bind _as_bp_third_person_character (Variables|Default|GetAs%20BP%20Third%20Person%20Character)
      (:then
        _)
      (:else
        (bind _asbp_third_person_character (Utilities|Casting|CastToBP_ThirdPersonCharacter OtherActor))
        (Variables|Default|SetAs%20BP%20Third%20Person%20Character _asbp_third_person_character)))
    (Variables|/Game/L_Content/Character/BP_ThirdPersonCharacter.BP_ThirdPersonCharacter_C|SetNearPushPullObject _as_bp_third_person_character true)
    (Variables|Default|SetisX?%20orY false)
    (Variables|/Game/L_Content/Character/BP_ThirdPersonCharacter.BP_ThirdPersonCharacter_C|SetBoxRotDirArrow (Variables|Default|GetAs%20BP%20Third%20Person%20Character) (Variables|Default|GetArrow2))))

(event OnComponentEndOverlap(collision)
  (params (OverlappedComponent :type Primitive%20Component%20Object%20Reference) (OtherActor :type Actor%20Object%20Reference) (OtherComp :type Primitive%20Component%20Object%20Reference) (OtherBodyIndex :type Integer))
  ;[1 1 1] final de overlap conn la pared sea al escalar por encima o al saltar
  (if (Actor|ActorHasTag OtherActor "Player")
    _))

(event OnComponentEndOverlap(collision1)
  (params (OverlappedComponent :type Primitive%20Component%20Object%20Reference) (OtherActor :type Actor%20Object%20Reference) (OtherComp :type Primitive%20Component%20Object%20Reference) (OtherBodyIndex :type Integer))
  ;[1 1 1] final de overlap conn la pared sea al escalar por encima o al saltar
  (if (Actor|ActorHasTag OtherActor "Player")
    _))

(event OnComponentEndOverlap(collision2)
  (params (OverlappedComponent :type Primitive%20Component%20Object%20Reference) (OtherActor :type Actor%20Object%20Reference) (OtherComp :type Primitive%20Component%20Object%20Reference) (OtherBodyIndex :type Integer))
  ;[1 1 1] final de overlap conn la pared sea al escalar por encima o al saltar
  (if (Actor|ActorHasTag OtherActor "Player")
    _))

(event OnComponentEndOverlap(collision3)
  (params (OverlappedComponent :type Primitive%20Component%20Object%20Reference) (OtherActor :type Actor%20Object%20Reference) (OtherComp :type Primitive%20Component%20Object%20Reference) (OtherBodyIndex :type Integer))
  ;[1 1 1] final de overlap conn la pared sea al escalar por encima o al saltar
  (if (Actor|ActorHasTag OtherActor "Player")
    _))

(event EventAxisMovement
  (params (XAxis :type Float%20%28double-precision%29) (YAxis :type Float%20%28double-precision%29))
  (bind _returnvalue (Utilities|Time|GetWorldDeltaSeconds))
  (bind _as_bp_third_person_character (Variables|Default|GetAs%20BP%20Third%20Person%20Character))
  (bind _as_bp_third_person_character_2 (Variables|Default|GetAs%20BP%20Third%20Person%20Character))
  (bind _sm (Variables|Default|GetSM))
  (bind _defaultsceneroot (Variables|Default|GetDefaultSceneRoot))
  (bind _defaultsceneroot_2 (Variables|Default|GetDefaultSceneRoot))
  (bind _returnvalue_2 (Transformation|GetWorldLocation _defaultsceneroot))
  (bind (_origin _boxextent) (Collision|GetComponentBounds _sm))
  (bind (_x _y _z) (Math|Vector|BreakVector _returnvalue_2))
  (bind (_x_2 _y_2 _z_2) (Math|Vector|BreakVector _returnvalue_2))
  (Variables|Default|SetAxisResult (+ XAxis YAxis))
  (Variables|Default|SetXAxis XAxis)
  (Variables|Default|SetYAxis (* YAxis -1.0))
  (Utilities|FlowControl|Sequence
    (:then_0
      ;[1 1 1] valor para la animacion retornar a 0 si no se esta empujando o tirando la caja
      (Utilities|FlowControl|RetriggerableDelay 0.5)
      (Variables|/Game/L_Content/Character/BP_ThirdPersonCharacter.BP_ThirdPersonCharacter_C|SetSelectAxisTovalueAnim (Variables|Default|GetAs%20BP%20Third%20Person%20Character) 0.0))
    (:then_1
      ;[1 1 1] Verificacion de colisiones en caso de bloqueo para poder tirar de la caja si colisiona de un lado con la algun objeto
      (if (Variables|Default|GetTraceCollision)
        (if (not (and (== (Variables|Default|GetLastIndexBlocked) (Variables|Default|GetIndexCollision)) (== (Variables|Default|GetLastAxisResult) (Variables|Default|GetAxisResult))))
          ;[1 1 1] Select segun el lado que haga overlap para seleccionar el axis a utilizar
          (bind _output_get (Variables|/Game/L_Content/Character/BP_ThirdPersonCharacter.BP_ThirdPersonCharacter_C|SetSelectAxisTovalueAnim (Variables|Default|GetAs%20BP%20Third%20Person%20Character) (Math|Float|SelectFloat (Variables|Default|GetXAxis) (Variables|Default|GetYAxis) (Variables|Default|GetisX?%20orY)) :!label _label))
          ;[1 1 1] al verificar en que axis vamos a mover la caja hace la interpolacion para el eje X o Y
          (if (Variables|Default|GetisX?%20orY)
            (Transformation|SetWorldLocation _defaultsceneroot_2 (Math|Interpolation|VInterptoConstant _returnvalue_2 (Math|Vector|MakeVector (.x (+ _returnvalue_2 (* _output_get (Variables|Default|GetSpeedMov)))) _y_2 _z_2) _returnvalue (Variables|Default|GetSpeedInterp)) false false)
            (else
              (Transformation|SetWorldLocation _defaultsceneroot_2 (Math|Interpolation|VInterptoConstant _returnvalue_2 (Math|Vector|MakeVector _x (Math|Float|Clamp(Float) (.y (+ _returnvalue_2 (* _output_get (Variables|Default|GetSpeedMov)))) (Variables|Default|GetclampMin) (Variables|Default|GetclampMax)) _z) _returnvalue (Variables|Default|GetSpeedInterp)) false false)))
          ;[1 1 1] creacion de box trace para detectar si esta colisionando con algun objeto
          (bind (_outhit _returnvalue_3) (Collision|BoxTraceByChannel (+ _origin (Variables|Default|GetoriginOffsetOverlap)) (+ (Math|Interpolation|VInterptoConstant _returnvalue_2 (Math|Vector|MakeVector (.x (+ _returnvalue_2 (* _output_get (Variables|Default|GetSpeedMov)))) _y_2 _z_2) _returnvalue (Variables|Default|GetSpeedInterp)) (* (* (Math|Vector|GetForwardVector (Variables|/Script/Engine.Actor|GetRootComponent _as_bp_third_person_character_2)) 2.0) (Variables|Default|GetAxisResult))) (* _boxextent (Variables|Default|GetMultiplyBoxExtend)) "0, 0, 0" "TraceTypeQuery1" false (Utilities|Array|MakeArray _as_bp_third_person_character_2) "ForOneFrame"))
          (bind _output_get_2 (Variables|Default|SetTraceCollision (and (.bInitialOverlap (Collision|BreakHitResult _outhit)) _returnvalue_3)))
          (if _output_get_2
            (Variables|Default|SetLastAxisResult (Variables|Default|GetAxisResult))
            (Variables|Default|SetLastIndexBlocked (Variables|Default|GetIndexCollision))))
        (else
          (goto _label))))
    (:then_2
      ;[1 1 1] mantener al character en la ubicacion del lado desde el que va  a empujar
      (Transformation|SetActorLocation _as_bp_third_person_character (Math|Interpolation|VInterptoConstant (Transformation|GetActorLocation _as_bp_third_person_character) (Transformation|GetWorldLocation (Utilities|Select :Index (Variables|Default|GetIndexCollision) :Option%200 (Variables|Default|GetArrow) :Option%201 (Variables|Default|GetArrow1) :Option%202 (Variables|Default|GetArrow2) :Option%203 (Variables|Default|GetArrow3))) (Utilities|Time|GetWorldDeltaSeconds) 2e+02) false false))))

(fn ConstructionScript)

(fn BolleansDeactivates
  (params (OwnerChar :type BP%20Third%20Person%20Character%20Object%20Reference) (NearPushPullObject :type Boolean) (PushingPulling :type Boolean) (TraceCollision :type Boolean) (CanMove :type Boolean))
  (Variables|/Game/L_Content/Character/BP_ThirdPersonCharacter.BP_ThirdPersonCharacter_C|SetNearPushPullObject OwnerChar NearPushPullObject)
  (Variables|/Game/L_Content/Character/BP_ThirdPersonCharacter.BP_ThirdPersonCharacter_C|SetPushingPulling OwnerChar PushingPulling)
  (Variables|Default|SetTraceCollision TraceCollision)
  (Variables|/Game/L_Content/Character/BP_ThirdPersonCharacter.BP_ThirdPersonCharacter_C|SetCanMove OwnerChar CanMove))