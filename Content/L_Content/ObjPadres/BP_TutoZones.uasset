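; BP_TutoZones is a tutorial trigger actor that shows mechanic hints when an actor tagged Player enters one of its six boxes.
; Each box overlap calls an event on a tutorial widget reference, passed in through the WBPTuto event, for push box, climb, carry or sprint.
; Two boxes share the carry hint, and Box4 only checks the tag without triggering anything.
; The construction script positions each box from its own relative location variable.
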(event OnComponentBeginOverlap(Box)
  (params (OverlappedComponent :type Primitive%20Component%20Object%20Reference) (OtherActor :type Actor%20Object%20Reference) (OtherComp :type Primitive%20Component%20Object%20Reference) (OtherBodyIndex :type Integer) (bFromSweep :type Boolean) (SweepResult :type Hit%20Result%20Structure%20%28by%20ref%29))
  (if (Actor|ActorHasTag OtherActor "Player")
    (Default|CEPushBox (Variables|Default|GetWBP%20Tuto) "xXXXXXXXXXXXXXXXXXXXXXXXXXXXXX")))

(event OnComponentBeginOverlap(Box1)
  (params (OverlappedComponent :type Primitive%20Component%20Object%20Reference) (OtherActor :type Actor%20Object%20Reference) (OtherComp :type Primitive%20Component%20Object%20Reference) (OtherBodyIndex :type Integer) (bFromSweep :type Boolean) (SweepResult :type Hit%20Result%20Structure%20%28by%20ref%29))
  (if (Actor|ActorHasTag OtherActor "Player")
    (Default|CEClimb (Variables|Default|GetWBP%20Tuto) "xXXXXXXXXXXXXXXXXXXXXXXXXXXXXX")))

(event OnComponentBeginOverlap(Box2)
  (params (OverlappedComponent :type Primitive%20Component%20Object%20Reference) (OtherActor :type Actor%20Object%20Reference) (OtherComp :type Primitive%20Component%20Object%20Reference) (OtherBodyIndex :type Integer) (bFromSweep :type Boolean) (SweepResult :type Hit%20Result%20Structure%20%28by%20ref%29))
  (if (Actor|ActorHasTag OtherActor "Player")
    (Default|CECarry (Variables|Default|GetWBP%20Tuto) "xXXXXXXXXXXXXXXXXXXXXXXXXXXXXX")))

(event OnComponentBeginOverlap(Box3)
  (params (OverlappedComponent :type Primitive%20Component%20Object%20Reference) (OtherActor :type Actor%20Object%20Reference) (OtherComp :type Primitive%20Component%20Object%20Reference) (OtherBodyIndex :type Integer) (bFromSweep :type Boolean) (SweepResult :type Hit%20Result%20Structure%20%28by%20ref%29))
  (if (Actor|ActorHasTag OtherActor "Player")
    (Default|CECarry (Variables|Default|GetWBP%20Tuto) "xXXXXXXXXXXXXXXXXXXXXXXXXXXXXX")))

(event OnComponentBeginOverlap(Box4)
  (params (OverlappedComponent :type Primitive%20Component%20Object%20Reference) (OtherActor :type Actor%20Object%20Reference) (OtherComp :type Primitive%20Component%20Object%20Reference) (OtherBodyIndex :type Integer) (bFromSweep :type Boolean) (SweepResult :type Hit%20Result%20Structure%20%28by%20ref%29))
  (if (Actor|ActorHasTag OtherActor "Player")
    _))

(event OnComponentBeginOverlap(Box5)
  (params (OverlappedComponent :type Primitive%20Component%20Object%20Reference) (OtherActor :type Actor%20Object%20Reference) (OtherComp :type Primitive%20Component%20Object%20Reference) (OtherBodyIndex :type Integer) (bFromSweep :type Boolean) (SweepResult :type Hit%20Result%20Structure%20%28by%20ref%29))
  (if (Actor|ActorHasTag OtherActor "Player")
    (Default|CESprint (Variables|Default|GetWBP%20Tuto) ">XXXXXXXXXXXXXXXXXXXXXXXXXXXXXXXXXXX")))

(event EventBeginPlay)

(event Collision|EventActorBeginOverlap
  (params (OtherActor :type Actor%20Object%20Reference)))

(event EventTick
  (params (DeltaSeconds :type Float%20%28single-precision%29)))

(event EventWBPTuto
  (params (WBP_Tuto :type WBP%20Tutorial%20Object%20Reference))
  (Variables|Default|SetWBP%20Tuto WBP_Tuto))

(fn ConstructionScript
  (Transformation|SetRelativeLocation (Variables|Default|GetBox) (Variables|Default|GetBoxLoc) false false)
  (Transformation|SetRelativeLocation (Variables|Default|GetBox1) (Variables|Default|GetBoxLoc1) false false)
  (Transformation|SetRelativeLocation (Variables|Default|GetBox2) (Variables|Default|GetBoxLoc2) false false)
  (Transformation|SetRelativeLocation (Variables|Default|GetBox3) (Variables|Default|GetBoxLoc3) false false)
  (Transformation|SetRelativeLocation (Variables|Default|GetBox4) (Variables|Default|GetBoxLoc4) false false)
  (Transformation|SetRelativeLocation (Variables|Default|GetBox5) (Variables|Default|GetBoxLoc5) false false))