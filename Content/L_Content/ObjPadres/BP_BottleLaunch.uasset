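; BP_BottleLaunch is a thrown bottle projectile that deals environmental radial damage, intended for the player, when its Hit event fires.
; The construction script drives the projectile movement's initial and max speed from the Impulso variable.
; Hit applies damage and spawns a Niagara effect at the hit location, then hides the mesh and disables collision to fake breakage before a delayed destroy.
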(event Collision|EventHit
  (params (MyComp :type Primitive%20Component%20Object%20Reference) (Other :type Actor%20Object%20Reference) (OtherComp :type Primitive%20Component%20Object%20Reference) (bSelfMoved :type Boolean) (HitLocation :type Vector :default "0, 0, 0") (HitNormal :type Vector :default "0, 0, 0") (NormalImpulse :type Vector :default "0, 0, 0") (Hit :type Hit%20Result%20Structure%20%28by%20ref%29))
  (bind _sm (Variables|Default|GetSM))
  ;[1 1 1] aplicar un daño radial que recibe el player
  (Game|Damage|ApplyRadialDamage 1e+01 HitLocation 2e+02 "/Engine/EngineDamageTypes/DmgTypeBP_Environmental.DmgTypeBP_Environmental_C" 0 self 0 false "ECC_Pawn")
  ;[1 1 1] creamos un efecto visual
  (Niagara|SpawnSystematLocation "/Game/Basic_VFX/Niagara/NS_Basic_6.NS_Basic_6" HitLocation "0, 0, 0" "2.000000,2.000000,2.000000")
  ;[1 1 1] quitamos la visibilidad de la botella y la colision para que parezca que se destruyo  se le quitan las colisiones
  (Rendering|SetVisibility _sm false false)
  (Collision|SetCollisionEnabled _sm "NoCollision")
  ;[1 1 1] En 4 segundos se destruye realmente ese actor en el mundo
  (Utilities|FlowControl|Delay 4.0)
  (Actor|DestroyActor))

(fn ConstructionScript
  (bind _projectilemovement (Variables|Default|GetProjectileMovement))
  (Variables|/Script/Engine.ProjectileMovementComponent|SetInitialSpeed _projectilemovement (Variables|Default|GetImpulso))
  (Variables|/Script/Engine.ProjectileMovementComponent|SetMaxSpeed _projectilemovement (Variables|Default|GetImpulso)))