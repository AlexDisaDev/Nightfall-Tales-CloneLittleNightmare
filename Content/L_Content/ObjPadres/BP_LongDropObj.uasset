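; BP_LongDropObj is a projectile object that the player can get and that makes noise when it hits something.
; Overlap events on its collision component set CanGetObj on the player-tagged BP_ThirdPersonCharacter on entry and clear it on exit.
; The Hit event calls MakeNoise at the impact location.
; The construction script applies InitialSpeed as both initial and maximum speed of its ProjectileMovement.
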(event OnComponentBeginOverlap(CollisionComponent)
  (params (OverlappedComponent :type Primitive%20Component%20Object%20Reference) (OtherActor :type Actor%20Object%20Reference) (OtherComp :type Primitive%20Component%20Object%20Reference) (OtherBodyIndex :type Integer) (bFromSweep :type Boolean) (SweepResult :type Hit%20Result%20Structure%20%28by%20ref%29))
  (if (Actor|ActorHasTag OtherActor "Player")
    (bind _asbp_third_person_character (Utilities|Casting|CastToBP_ThirdPersonCharacter OtherActor))
    (Variables|/Game/L_Content/Character/BP_ThirdPersonCharacter.BP_ThirdPersonCharacter_C|SetcanGetObj? _asbp_third_person_character true)))

(event OnComponentEndOverlap(CollisionComponent)
  (params (OverlappedComponent :type Primitive%20Component%20Object%20Reference) (OtherActor :type Actor%20Object%20Reference) (OtherComp :type Primitive%20Component%20Object%20Reference) (OtherBodyIndex :type Integer))
  (if (Actor|ActorHasTag OtherActor "Player")
    (bind _asbp_third_person_character (Utilities|Casting|CastToBP_ThirdPersonCharacter OtherActor))
    (Variables|/Game/L_Content/Character/BP_ThirdPersonCharacter.BP_ThirdPersonCharacter_C|SetcanGetObj? _asbp_third_person_character false)))

(event EventBeginPlay)

(event Collision|EventHit
  (params (MyComp :type Primitive%20Component%20Object%20Reference) (Other :type Actor%20Object%20Reference) (OtherComp :type Primitive%20Component%20Object%20Reference) (bSelfMoved :type Boolean) (HitLocation :type Vector :default "0, 0, 0") (HitNormal :type Vector :default "0, 0, 0") (NormalImpulse :type Vector :default "0, 0, 0") (Hit :type Hit%20Result%20Structure%20%28by%20ref%29))
  (Class|Actor|MakeNoise 1.0 0 HitLocation 0.0 "None"))

(fn ConstructionScript
  (bind _projectilemovement (Variables|MyProjectile|GetProjectileMovement))
  (bind _initial_speed (Variables|Default|GetInitial%20Speed))
  (Variables|/Script/Engine.ProjectileMovementComponent|SetInitialSpeed _projectilemovement _initial_speed)
  (Variables|/Script/Engine.ProjectileMovementComponent|SetMaxSpeed _projectilemovement _initial_speed))