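; BP_Trap is a trap actor that slides its mesh vertically when the player triggers it and kills the player on contact with its kill box.
; Box1 overlap by a Player-tagged actor starts a looping timer that moves the mesh toward ValueZ at constant speed, clearing itself on arrival.
; Box overlap calls CEDead on BP_ThirdPersonCharacter.
; The mesh's starting position is saved at BeginPlay but never used here.
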(event OnComponentBeginOverlap(Box)
  (params (OverlappedComponent :type Primitive%20Component%20Object%20Reference) (OtherActor :type Actor%20Object%20Reference) (OtherComp :type Primitive%20Component%20Object%20Reference) (OtherBodyIndex :type Integer) (bFromSweep :type Boolean) (SweepResult :type Hit%20Result%20Structure%20%28by%20ref%29))
  ;[1 1 1] para aviso de trampa
  (if (Actor|ActorHasTag OtherActor "Player")
    (bind _asbp_third_person_character (Utilities|Casting|CastToBP_ThirdPersonCharacter OtherActor))
    (Default|CEDead _asbp_third_person_character)))

(event OnComponentBeginOverlap(Box1)
  (params (OverlappedComponent :type Primitive%20Component%20Object%20Reference) (OtherActor :type Actor%20Object%20Reference) (OtherComp :type Primitive%20Component%20Object%20Reference) (OtherBodyIndex :type Integer) (bFromSweep :type Boolean) (SweepResult :type Hit%20Result%20Structure%20%28by%20ref%29))
  (if (Actor|ActorHasTag OtherActor "Player")
    (bind _returnvalue (Utilities|Time|SetTimerbyEvent (delegate Custom|CE_ActivateTrap) 0.01 true))
    (Variables|Default|SethandleTrapTimer _returnvalue)))

(event Custom|CE_ActivateTrap
  (bind _returnvalue (Utilities|Time|GetWorldDeltaSeconds))
  (bind _staticmesh (Variables|Default|GetStaticMesh))
  (bind _valuez (Variables|Default|GetValueZ))
  (bind _returnvalue_2 (Transformation|GetWorldLocation _staticmesh))
  (bind _returnvalue_3 (Math|Interpolation|FInterptoConstant (.z _returnvalue_2) _valuez _returnvalue 4e+02))
  (Transformation|SetWorldLocation _staticmesh (Math|Vector|MakeVector (.x _returnvalue_2) (.y _returnvalue_2) _returnvalue_3) false false)
  (if (== (Math|Float|Truncate _returnvalue_3) (Math|Float|Truncate (Variables|Default|GetValueZ)))
    (Utilities|Time|ClearandInvalidateTimerbyHandle (Variables|Default|GethandleTrapTimer))))

(event EventBeginPlay
  (Variables|Default|SetFirstPosition (Transformation|GetWorldLocation (Variables|Default|GetStaticMesh))))

(fn ConstructionScript)