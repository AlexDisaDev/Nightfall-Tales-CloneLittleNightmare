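; BP_Ladder is a ladder actor that tells the player's BP_ThirdPersonCharacter when it can climb.
; Two trigger boxes each flag a tagged player as near the ladder and pass their own arrow as the climb rotation reference.
; Leaving either box clears the near and on-ladder flags and restores walking movement.
; The climbing itself is left to the character, and the construction script does nothing.
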(event OnComponentBeginOverlap(Box)
  (params (OverlappedComponent :type Primitive%20Component%20Object%20Reference) (OtherActor :type Actor%20Object%20Reference) (OtherComp :type Primitive%20Component%20Object%20Reference) (OtherBodyIndex :type Integer) (bFromSweep :type Boolean) (SweepResult :type Hit%20Result%20Structure%20%28by%20ref%29))
  ;[1 1 1] overlap para detectar pared  para escalar e interactuar desde el character y obtener la rotacion para el personaje
  (if (Actor|ActorHasTag OtherActor "Player")
    (bind _asbp_third_person_character (Utilities|Casting|CastToBP_ThirdPersonCharacter OtherActor))
    (Variables|/Game/L_Content/Character/BP_ThirdPersonCharacter.BP_ThirdPersonCharacter_C|SetNear%20Ladder _asbp_third_person_character true)
    (Variables|/Game/L_Content/Character/BP_ThirdPersonCharacter.BP_ThirdPersonCharacter_C|SetladdderRotDirActor _asbp_third_person_character (Variables|Default|GetArrow))))

(event OnComponentEndOverlap(Box)
  (params (OverlappedComponent :type Primitive%20Component%20Object%20Reference) (OtherActor :type Actor%20Object%20Reference) (OtherComp :type Primitive%20Component%20Object%20Reference) (OtherBodyIndex :type Integer))
  ;[1 1 1] overlap para detectar pared  para escalar e interactuar desde el character y obtener la rotacion para el personaje
  (if (Actor|ActorHasTag OtherActor "Player")
    (bind _asbp_third_person_character (Utilities|Casting|CastToBP_ThirdPersonCharacter OtherActor))
    (Variables|/Game/L_Content/Character/BP_ThirdPersonCharacter.BP_ThirdPersonCharacter_C|SetNear%20Ladder _asbp_third_person_character false)
    (Variables|/Game/L_Content/Character/BP_ThirdPersonCharacter.BP_ThirdPersonCharacter_C|SetOnLadder _asbp_third_person_character false)
    (Pawn|Components|CharacterMovement|SetMovementMode (Variables|/Script/Engine.Character|GetCharacterMovement _asbp_third_person_character) "MOVE_Walking" 0)))

(event OnComponentBeginOverlap(Box1)
  (params (OverlappedComponent :type Primitive%20Component%20Object%20Reference) (OtherActor :type Actor%20Object%20Reference) (OtherComp :type Primitive%20Component%20Object%20Reference) (OtherBodyIndex :type Integer) (bFromSweep :type Boolean) (SweepResult :type Hit%20Result%20Structure%20%28by%20ref%29))
  ;[1 1 1] overlap para detectar pared  para escalar e interactuar desde el character y obtener la rotacion para el personaje
  (if (Actor|ActorHasTag OtherActor "Player")
    (bind _asbp_third_person_character (Utilities|Casting|CastToBP_ThirdPersonCharacter OtherActor))
    (Variables|/Game/L_Content/Character/BP_ThirdPersonCharacter.BP_ThirdPersonCharacter_C|SetNear%20Ladder _asbp_third_person_character true)
    (Variables|/Game/L_Content/Character/BP_ThirdPersonCharacter.BP_ThirdPersonCharacter_C|SetladdderRotDirActor _asbp_third_person_character (Variables|Default|GetArrow1))))

(event OnComponentEndOverlap(Box1)
  (params (OverlappedComponent :type Primitive%20Component%20Object%20Reference) (OtherActor :type Actor%20Object%20Reference) (OtherComp :type Primitive%20Component%20Object%20Reference) (OtherBodyIndex :type Integer))
  ;[1 1 1] overlap para detectar pared  para escalar e interactuar desde el character y obtener la rotacion para el personaje
  (if (Actor|ActorHasTag OtherActor "Player")
    (bind _asbp_third_person_character (Utilities|Casting|CastToBP_ThirdPersonCharacter OtherActor))
    (Variables|/Game/L_Content/Character/BP_ThirdPersonCharacter.BP_ThirdPersonCharacter_C|SetNear%20Ladder _asbp_third_person_character false)
    (Variables|/Game/L_Content/Character/BP_ThirdPersonCharacter.BP_ThirdPersonCharacter_C|SetOnLadder _asbp_third_person_character false)
    (Pawn|Components|CharacterMovement|SetMovementMode (Variables|/Script/Engine.Character|GetCharacterMovement _asbp_third_person_character) "MOVE_Walking" 0)))

(fn ConstructionScript)