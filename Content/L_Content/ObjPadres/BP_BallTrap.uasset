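; BP_BallTrap is a trap actor that releases a physics ball when an actor tagged "Player" enters its trigger box.
; The construction script applies exposed settings for ramp transform and visibility, ball position, scale and initial physics, and box scale.
; On overlap, the box unhides the ball and enables its physics simulation, although the construction script already sets the ball visible.
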(event OnComponentBeginOverlap(Box)
  (params (OverlappedComponent :type Primitive%20Component%20Object%20Reference) (OtherActor :type Actor%20Object%20Reference) (OtherComp :type Primitive%20Component%20Object%20Reference) (OtherBodyIndex :type Integer) (bFromSweep :type Boolean) (SweepResult :type Hit%20Result%20Structure%20%28by%20ref%29))
  (if (Actor|ActorHasTag OtherActor "Player")
    (Development|SetHiddeninGame (Variables|Default|GetBAll) false false)
    (Physics|SetSimulatePhysics (Variables|Default|GetBAll) true)
    (Physics|SetSimulatePhysics (Variables|Default|GetBAll) true)))

(event EventBeginPlay)

(event Collision|EventActorBeginOverlap
  (params (OtherActor :type Actor%20Object%20Reference)))

(event EventTick
  (params (DeltaSeconds :type Float%20%28single-precision%29)))

(fn ConstructionScript
  (bind _ramp (Variables|Default|Getramp))
  (bind _ball (Variables|Default|GetBAll))
  (Transformation|SetRelativeLocation _ramp (Variables|Default|GetRampLocation) false false)
  (Transformation|SetRelativeRotation _ramp (Variables|Default|GetRampRotation) false false)
  (Development|SetHiddeninGame _ramp (Variables|Default|GetRampHiddenInGame) false)
  (Transformation|SetRelativeLocation _ball (Variables|Default|GetBalllocation) false false)
  (Transformation|SetWorldScale3D _ball (Variables|Default|GetBallScale))
  (Physics|SetSimulatePhysics _ball (Variables|Default|GetBallSimulate^hysiscs))
  (Development|SetHiddeninGame _ball false false)
  (Transformation|SetWorldScale3D (Variables|Default|GetBox) (Variables|Default|GetBoxScale)))