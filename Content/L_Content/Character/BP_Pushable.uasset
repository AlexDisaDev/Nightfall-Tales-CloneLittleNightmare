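; BP_Pushable is a pushable object with a configurable mesh and a list of push transforms, shown as arrow components by the construction script.
; FindClosestPushTransform picks the index of the transform nearest a character within push range, using squared 2D distances.
; The Hold event calls HandleInteraction, which is unfinished: its validation and lookup logic is disconnected, so holding currently does nothing.
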(event EventHold
  (params (Character :type Character%20Object%20Reference))
  (CallFunction|HandleInteraction Character))

(fn ConstructionScript
  (Components|StaticMesh|SetStaticMesh (Variables|Default|GetStaticMesh) (Variables|Default|GetNewMesh))
  (for _array_element (Variables|Default|GetPush%20Transform)
    (AddComponent|AddArrowComponent false _array_element)))

(fn HandleInteraction
  (params (Character :type Character%20Object%20Reference)))

(fn FindClosestPushTransform
  (params (CharacterLocation :type Vector%202D%20Structure) (PushRange :type Float%20%28double-precision%29))
  (for (_array_element _array_index) (Variables|Default|GetPush%20Transform)
    (LocalVariables|SetCurrentTransform _array_index)
    (LocalVariables|SetCurrentDistance (Class|KismetMathLibrary|DistanceSquared2D (Math|Conversions|ToVector2D(Vector) (Math|Transform|TransformLocation (Transformation|GetActorTransform) (.location _array_element))) CharacterLocation))
    (if (< (LocalVariables|GetCurrentDistance) (Math|Float|Square PushRange))
      (if (or (< (LocalVariables|GetCurrentDistance) (LocalVariables|GetClosestDistance)) (< (LocalVariables|GetClosestTransform) 0))
        (LocalVariables|SetClosestTransform (LocalVariables|GetCurrentTransform))
        (LocalVariables|SetClosestDistance (LocalVariables|GetCurrentDistance)))))
  (return (LocalVariables|GetClosestTransform)))