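; Game mode that shows a loading screen at BeginPlay, gates player input and handles respawning.
; PostLogin stores the controller and disables its pawn's input, and CE_EnableInputs restores it, both retrying on a short delay until a pawn is valid.
; CE_Respawn spawns a new third-person character at LocToSpawn, or the first PlayerStart if that is zero, then possesses it with player controller 0 and calls its CERespawn.
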(event Custom|CE_Respawn
  (if (Utilities|Operators|NotEqual(!=) :A (Variables|Default|GetLocToSpawn))
    (bind _returnvalue (Game|SpawnActorfromClass "/Game/L_Content/Character/BP_ThirdPersonCharacter.BP_ThirdPersonCharacter_C" (Math|Transform|MakeTransform (Variables|Default|GetLocToSpawn) "0, 0, 0" "1.000000,1.000000,1.000000") "Undefined" "MultiplyWithRoot" 0 0))
    (Pawn|Possess (Game|GetPlayerController 0) _returnvalue)
    (Default|CERespawn _returnvalue)
    (else
      (bind _outactors (Actor|GetAllActorsOfClass "/Script/Engine.PlayerStart"))
      (bind _returnvalue_2 (Game|SpawnActorfromClass "/Game/L_Content/Character/BP_ThirdPersonCharacter.BP_ThirdPersonCharacter_C" (Math|Transform|MakeTransform (Transformation|GetActorLocation (Utilities|Array|Get(acopy) _outactors)) "0, 0, 0" "1.000000,1.000000,1.000000") "Undefined" "MultiplyWithRoot" 0 0))
      (Pawn|Possess (Game|GetPlayerController 0) _returnvalue_2)
      (Default|CERespawn _returnvalue_2))))

(event Custom|CE_EnableInputs
  (bind _controller (Variables|Default|GetController))
  (bind _returnvalue (Pawn|GetControlledPawn _controller))
  (Utilities|IsValid _returnvalue :!label _label
    (:Is%20Valid
      (Input|EnableInput _returnvalue _controller))
    (:Is%20Not%20Valid
      (Utilities|FlowControl|Delay 0.2)
      (goto _label))))

(event EventBeginPlay
  (bind _returnvalue (UserInterface|CreateWidget "/Game/L_Content/Widgets/WBP/WBP_LoadingScreen.WBP_LoadingScreen_C"))
  (bind _output_get (Variables|Default|SetWBP _returnvalue))
  (UserInterface|Viewport|AddtoViewport _returnvalue 0)
  (Default|CELoadingBar (Variables|Default|GetWBP)))

(event EventTick
  (params (DeltaSeconds :type Float%20%28single-precision%29)))

(event EventPostLogin
  (params (NewPlayer :type Player%20Controller%20Object%20Reference))
  (bind _returnvalue (Pawn|GetControlledPawn NewPlayer))
  (Utilities|IsValid _returnvalue :!label _label
    (:Is%20Valid
      (Variables|Default|SetController NewPlayer)
      (Input|DisableInput _returnvalue NewPlayer))
    (:Is%20Not%20Valid
      (Utilities|FlowControl|Delay 0.2)
      (goto _label))))

(fn ConstructionScript)